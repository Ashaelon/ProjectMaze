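; Actor component that makes its owner's light flicker, along with an optional particle system and attached sound events.
; BeginPlay caches the components it finds and enables ticking if any exist.
; Tick uses random delays, weighting and a visibility mode to pick an intensity that drives light brightness and sound volume.
; An emit mode switches particles and their sound by that intensity or randomly, though the Maximum check is unwired.
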(event EventBeginPlay
  (bind _returnvalue (Components|GetOwner))
  (bind _lightsound (Variables|Default|GetLightSound))
  (bind _particlesystemsound (Variables|Default|GetParticleSystemSound))
  (bind _returnvalue_2 (Actor|GetComponentbyClass _returnvalue "/Script/Engine.LightComponent"))
  (bind _returnvalue_3 (Actor|GetComponentbyClass _returnvalue "/Script/Engine.ParticleSystemComponent"))
  ;[1 1 1] Set up components
  ;;[1 1 1] Get Owner
  (Utilities|IsValid _returnvalue
    (:Is%20Valid
      (Utilities|FlowControl|Sequence
        (:then_0
          ;;[1 1 1] Get Owner Light Component
          (Utilities|IsValid _returnvalue_2
            (:Is%20Valid
              (bind _output_get (Variables|Default|SetLight _returnvalue_2))
              (Rendering|Components|Light|SetIntensity _output_get (Variables|Default|GetmaxIntensity))
              (Variables|Default|SetcanEnableTick true :!label _label))))
        (:then_1
          ;;[1 1 1] Set sound component for light
          (Utilities|IsValid _lightsound
            (:Is%20Valid
              (bind _returnvalue_4 (Class|FMODBlueprintStatics|PlayEventAttached _lightsound (Actor|GetComponentbyClass _returnvalue "/Script/Engine.SceneComponent") "None" "0, 0, 0" "KeepRelativeOffset" false false))
              (Variables|Default|SetLightSoundComponent _returnvalue_4)
              (goto _label))))
        (:then_2
          ;;[1 1 1] Get Particle System
          (Utilities|IsValid _returnvalue_3
            (:Is%20Valid
              (Variables|Default|SetParticleSystemComponent _returnvalue_3)
              (goto _label))))
        (:then_3
          ;;[1 1 1] Set sound for particle system
          (Utilities|IsValid _particlesystemsound
            (:Is%20Valid
              (bind _returnvalue_5 (Class|FMODBlueprintStatics|PlayEventAttached _particlesystemsound (Actor|GetComponentbyClass _returnvalue "/Script/Engine.SceneComponent") "None" "0, 0, 0" "KeepRelativeOffset" false false))
              (bind _output_get_2 (Variables|Default|SetParticleSystemSoundComponent _returnvalue_5))
              (Class|FMODAudioComponent|SetVolume _output_get_2 (Math|Conversions|ToFloat(Integer) (Variables|Default|GetmaxParticleSoundVolume)))
              (goto _label))))
        (:then_4
          ;;[1 1 1] Enable tick
          (Components|Tick|SetComponentTickEnabled (Variables|Default|GetcanEnableTick)))))))

(event EventTick
  (params (DeltaSeconds :type Float%20%28single-precision%29))
  (bind _returnvalue (Math|Random|RandomFloatinRange 0.2 0.9))
  (bind _particlesystemcomponent (Variables|Default|GetParticleSystemComponent))
  (bind _light (Variables|Default|GetLight))
  (bind _lightsoundcomponent (Variables|Default|GetLightSoundComponent))
  (bind _particlesystemsoundcomponent (Variables|Default|GetParticleSystemSoundComponent))
  (bind _minintensity (Variables|Default|GetminIntensity))
  (bind _maxintensity (Variables|Default|GetmaxIntensity))
  ;[1 1 1] Flicker Control
  (Utilities|FlowControl|Sequence
    (:then_0
      ;;[1 1 1] Set flicker intensity (does not need a light component)
      (Utilities|FlowControl|Delay (Math|Random|RandomFloatinRange 0.0 (Variables|Default|GetmaxDelay)))
      (if (Math|Random|RandomBoolwithWeight (Variables|Default|Getweight))
        (Variables|Default|Setintensity (Math|Random|RandomFloatinRange _minintensity _maxintensity) :!label _label)
        (else
          (switch Utilities|FlowControl|Switch|SwitchonELightVisibility (Variables|Default|GetlightVisibility)
            (:NewEnumerator0
              (goto _label))
            (:NewEnumerator1
              (Variables|Default|Setintensity _maxintensity))
            (:NewEnumerator2
              (Variables|Default|Setintensity _minintensity))))))
    (:then_1
      ;;[1 1 1] Set light intensity if light component exists
      (Utilities|IsValid _light
        (:Is%20Valid
          (Rendering|Components|Light|SetIntensity _light (Variables|Default|Getintensity)))))
    (:then_2
      ;;[1 1 1] Set light sound flicker
      (Utilities|IsValid _lightsoundcomponent
        (:Is%20Valid
          (Class|FMODAudioComponent|SetVolume _lightsoundcomponent (* (Variables|Default|GetmaxLightSoundVolume) (/ (Variables|Default|Getintensity) (Variables|Default|GetmaxIntensity))))
          (bind _returnvalue_2 (Class|FMODAudioComponent|IsPlaying _lightsoundcomponent))
          (if (not _returnvalue_2)
            (Class|FMODAudioComponent|Play _lightsoundcomponent)))))
    (:then_3
      ;;[1 1 1] Set particle system flicker if particle system exists
      (Utilities|IsValid _particlesystemcomponent
        (:Is%20Valid
          (switch Utilities|FlowControl|Switch|SwitchonEParticleSystemEmit (Variables|Default|GetparticleSystemEmit)
            (:NewEnumerator0
              (Components|Activation|Activate _particlesystemcomponent false :!label _label_2)
              (Variables|Default|SetcanPlaySound true))
            (:NewEnumerator1
              (Components|Activation|Deactivate _particlesystemcomponent :!label _label_3)
              (Variables|Default|SetcanPlaySound false))
            (:NewEnumerator2
              (Utilities|EqualTo(Max)
                (:True
                  (goto _label_2))
                (:False
                  (goto _label_3))))
            (:NewEnumerator3
              (Utilities|EqualTo(Min)
                (:True
                  (goto _label_2))
                (:False
                  (goto _label_3))))
            (:NewEnumerator4
              (Utilities|IsLessThan
                (:True
                  (goto _label_2))
                (:False
                  (goto _label_3))))
            (:NewEnumerator5
              (Utilities|IsGreaterThan
                (:True
                  (goto _label_2))
                (:False
                  (goto _label_3))))
            (:NewEnumerator6
              (Utilities|FlowControl|Delay _returnvalue :!label _label_4)
              (if (Math|Random|RandomBool)
                (Components|Activation|Activate _particlesystemcomponent false)
                (Variables|Default|SetcanPlaySound true)
                (Utilities|FlowControl|Delay _returnvalue)
                (goto _label_3)))
            (:NewEnumerator7
              (Utilities|IsLessThan
                (:True
                  (goto _label_4))
                (:False
                  (goto _label_3))))
            (:NewEnumerator8
              (Utilities|IsGreaterThan
                (:True
                  (goto _label_4))
                (:False
                  (goto _label_3))))))))
    (:then_4
      (if (Variables|Default|GetcanPlaySound)
        (Utilities|IsValid _particlesystemsoundcomponent
          (:Is%20Valid
            ;;[1 1 1] Play particle system sound
            (bind _returnvalue_3 (Class|FMODAudioComponent|IsPlaying _particlesystemsoundcomponent))
            (if (not _returnvalue_3)
              (Class|FMODAudioComponent|Play _particlesystemsoundcomponent))))
        (else
          (Utilities|IsValid _particlesystemsoundcomponent
            (:Is%20Valid
              ;;[1 1 1] Stop particle system sound
              (bind _returnvalue_4 (Class|FMODAudioComponent|IsPlaying _particlesystemsoundcomponent))
              (if _returnvalue_4
                (Class|FMODAudioComponent|Stop _particlesystemsoundcomponent)))))))))

(fn PlayParticleSound
  (params (PlaySound :type Boolean)))

(fn FlickerParticleSystem)